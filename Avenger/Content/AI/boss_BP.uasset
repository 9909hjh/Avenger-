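; Boss enemy AI pawn that chases the first Katana actor in the level and attacks it at close range.
; After a short delay it stores that actor as MyBoss and sets AI controller focus on it.
; BaseMovement loops AIMoveTo toward the target, pausing after each successful move.
; AttackRange overlap starts the samurai attack montage, which replays on completion until the target leaves the range.
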(event `self.ReceiveBeginPlay`
  (`|ExecutionSequence`
    (:`then_0`
      (`self.GetBoss`))
    (:`then_1`
      (`self.BaseMovement`))
    (:`then_2`
      (bind _asai_controller_boss_bp (cast `/Game/AI/AI_Controller_boss_BP` (`self.GetController`)))
      (set `self.AIController` _asai_controller_boss_bp))))

(event `GetBoss`
  (`KismetSystemLibrary.Delay` 1.0)
  (bind _outactors (`GameplayStatics.GetAllActorsOfClass` "/Game/ju-hyeong/Katana.Katana_C"))
  (set `self.MyBoss` (`|GetArrayItem` _outactors))
  (`AIController.K2_SetFocus` (`self.AIController`) (`self.MyBoss`)))

(event `BaseMovement`
  (`/Engine/EditorBlueprintResources/StandardMacros.IsValid` (`self.MyBoss`) :!label _label
    (:`Is Valid`
      (`|AIMoveTo` self (0.0 0.0 0.0) (`self.MyBoss`) 50.0
        (:`OnSuccess`
          (`KismetSystemLibrary.Delay` 3.0)
          (goto _label))))
    (:`Is Not Valid`
      (`KismetSystemLibrary.Delay` 1.0)
      (goto _label))))

(event `self.AttackRange.OnComponentBeginOverlap`
  (params (OverlappedComponent :type "PrimitiveComponent Object Reference") (OtherActor :type "Actor Object Reference") (OtherComp :type "PrimitiveComponent Object Reference") (OtherBodyIndex :type Integer) (bFromSweep :type Boolean) (SweepResult :type "HitResult Structure (by ref)"))
  (if (and (== OtherActor (`self.MyBoss`)) (not (`self.IsAttacking`)))
    (set `self.CanAttack` true)
    (set `self.IsAttacking` true :!label _label_2)
    (`|PlayMontage` (`self.Mesh`) "/Game/AI/Anim_Samurai_Boss_attack_Montage.Anim_Samurai_Boss_attack_Montage"
      (:`OnCompleted`
        (set `self.IsAttacking` false)
        (if (`self.CanAttack`)
          (goto _label_2))))))

(event `self.AttackRange.OnComponentEndOverlap`
  (params (OverlappedComponent :type "PrimitiveComponent Object Reference") (OtherActor :type "Actor Object Reference") (OtherComp :type "PrimitiveComponent Object Reference") (OtherBodyIndex :type Integer))
  (if (and (== OtherActor (`self.MyBoss`)) (`self.CanAttack`))
    (set `self.CanAttack` false)))

(fn `UserConstructionScript`)